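; Cube actor variant that wanders within a rectangular XY zone centered on its starting position.
; Tick sweeps it forward at Speed and calls Return when it leaves the zone, re-aiming it at a random point inside.
; A looping timer also picks new random headings while in bounds.
; Hit re-aims it on collision, using a DoOnce and short Delay as a cooldown.
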(event Custom|Rotate
  ;[1 1 1] random rotation of the cube to a point in the zone
  (if (CallFunction|IsActorinBoundires2D (Variables|Default|GetMIN_X) (Variables|Default|GetMAX_X) (Variables|Default|GetMIN_Y) (Variables|Default|GetMAX_Y))
    (Transformation|SetActorRotation (Math|Rotator|FindLookatRotation (Variables|/Script/Engine.SceneComponent|GetRelativeLocation (Variables|Default|GetCube)) (Math|Random|RandomPointinBoundingBox (stale EventBeginPlay _output_get) (Math|Vector|MakeVector (Variables|Default|GetMAX_X) (Variables|Default|GetMAX_Y) 0.0))))))

(event Custom|Return
  ;[1 1 1] Return cub is zone
  (if (CallFunction|IsActorinBoundires2D (Variables|Default|GetMIN_X) (Variables|Default|GetMAX_X) (Variables|Default|GetMIN_Y) (Variables|Default|GetMAX_Y))
    (goto _label Reset)
    (else
      (Utilities|FlowControl|DoOnce false :!label _label
        (:Completed
          (Transformation|SetActorRotation (Math|Rotator|FindLookatRotation (Variables|/Script/Engine.SceneComponent|GetRelativeLocation (Variables|Default|GetCube)) (Math|Random|RandomPointinBoundingBox (Variables|Default|GetCurrentObjectLocation) (Math|Vector|MakeVector (Variables|Default|GetMAX_X) (Variables|Default|GetMAX_Y) 0.0))))
          (goto _label Reset))))))

(event EventTick
  (params (DeltaSeconds :type Float%20%28single-precision%29))
  ;[1 1 1] Cube Movement var1
  (Transformation|SetActorLocation (+ (* (Math|Vector|GetForwardVector (Variables|Default|GetCube)) (* DeltaSeconds (Variables|Default|GetSpeed))) (Transformation|GetActorLocation)) true false)
  ;[1 1 1] checking coordinates
  (if (not (CallFunction|IsActorinBoundires2D (Variables|Default|GetMIN_X) (Variables|Default|GetMAX_X) (Variables|Default|GetMIN_Y) (Variables|Default|GetMAX_Y)))
    (CallFunction|Return)))

(event EventBeginPlay
  ;[1 1 1] setting the coordinates of the zone center(var1)
  (bind _output_get (Variables|Default|SetCurrentObjectLocation (Transformation|GetWorldLocation (Variables|Default|GetCube))))
  ;[1 1 1] random rotation of the cube to a point in the zone
  (Utilities|Time|SetTimerbyEvent (delegate Custom|Rotate) 2.0 true))

(event Collision|EventHit
  (params (MyComp :type Primitive%20Component%20Object%20Reference) (Other :type Actor%20Object%20Reference) (OtherComp :type Primitive%20Component%20Object%20Reference) (bSelfMoved :type Boolean) (HitLocation :type Vector :default "0, 0, 0") (HitNormal :type Vector :default "0, 0, 0") (NormalImpulse :type Vector :default "0, 0, 0") (Hit :type Hit%20Result%20Structure%20%28by%20ref%29))
  (bind _max_y (Variables|Default|GetMAX_Y))
  (bind _max_x (Variables|Default|GetMAX_X))
  (bind _currentobjectlocation (Variables|Default|GetCurrentObjectLocation))
  (bind _cube (Variables|Default|GetCube))
  (bind _returnvalue (Math|Random|RandomPointinBoundingBox _currentobjectlocation (Math|Vector|MakeVector _max_x _max_y 0.0)))
  (bind _relativelocation (Variables|/Script/Engine.SceneComponent|GetRelativeLocation _cube))
  (bind _returnvalue_2 (Math|Rotator|FindLookatRotation _relativelocation _returnvalue))
  ;[1 1 1] cube rotation on collision
  (Utilities|FlowControl|DoOnce false :!label _label
    (:Completed
      (Transformation|SetActorRotation (Math|Rotator|MakeRotator (.roll _returnvalue_2) (.pitch _returnvalue_2) (.yaw _returnvalue_2)) true)
      (Utilities|FlowControl|Delay 0.2)
      (goto _label Reset))))

(fn ConstructionScript)

(fn IsActorinBoundires2D
  (params (MIN_X :type Float%20%28double-precision%29) (MAX_X :type Float%20%28double-precision%29) (MIN_Y :type Float%20%28double-precision%29) (MAX_Y :type Float%20%28double-precision%29))
  (bind _returnvalue (Transformation|GetActorLocation))
  (bind _currentobjectlocation (Variables|Default|GetCurrentObjectLocation))
  ;[1 1 1] Settings coordinats zone
  (return (and (Math|Float|InRange(Float) (.x _returnvalue) (+ MIN_X (.x _currentobjectlocation)) (+ MAX_X (.x _currentobjectlocation))) (Math|Float|InRange(Float) (.y _returnvalue) (+ MIN_Y (.y _currentobjectlocation)) (+ MAX_Y (.y _currentobjectlocation))))))