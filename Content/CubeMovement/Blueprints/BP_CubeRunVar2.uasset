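; Cube pawn that wanders endlessly on the navmesh, kept near a rectangular zone centered on its BeginPlay location.
; MoveToTarget checks the zone with IsActorInBoundires2D; inside, it faces a random reachable nearby point and runs AI MoveTo, looping on success or failure.
; Outside, it moves to a random point in the zone box, retrying on failure; facing and destination use separate random calls, so they can differ.
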(event Custom|MoveToTarget
  (bind _max_y (Variables|Default|GetMAX_Y))
  (bind _currentobjectlocation (Variables|Default|GetCurrentObjectLocation))
  (bind _max_x (Variables|Default|GetMAX_X))
  (bind _returnvalue (Math|Random|RandomPointinBoundingBox _currentobjectlocation (Math|Vector|MakeVector _max_x _max_y 0.0)))
  ;[1 1 1] checking coordinates
  (bind _bisinbounds (CallFunction|IsActorinBoundires2D (Variables|Default|GetMIN_X) (Variables|Default|GetMAX_X) (Variables|Default|GetMIN_Y) (Variables|Default|GetMAX_Y)))
  (if _bisinbounds
    ;[1 1 1] Cube Movement var2
    (bind _output_get (Variables|Default|SetTargetLocation (.RandomLocation (AI|Navigation|GetRandomReachablePointinRadius (Transformation|GetActorLocation) 6e+02 0 0))))
    (Transformation|SetActorRotation (Math|Rotator|FindLookatRotation (Transformation|GetWorldLocation (Variables|Default|GetCube)) _output_get))
    (bind _movementresult (AI|AIMoveTo self (Variables|Default|GetTargetLocation) 0 5.0 false)
      (:OnSuccess
        ;[1 1 1] further customization possibility
        (switch Utilities|FlowControl|Switch|SwitchonEPathFollowingResult _movementresult
          (:Success
            _)))
      (:OnFail
        _))
    (else
      ;[1 1 1] Return cub is zone
      (Transformation|SetActorRotation (Math|Rotator|FindLookatRotation (Transformation|GetWorldLocation (Variables|Default|GetCube)) (Math|Vector|MakeVector (.x _returnvalue) (.y _returnvalue) 0.0)) :!label _label)
      (AI|AIMoveTo self (Math|Vector|MakeVector (.x _returnvalue) (.y _returnvalue) 0.0) 0 5.0 false
        (:OnSuccess
          _)
        (:OnFail
          (goto _label)))))
  (CallFunction|MovetoTarget))

(event EventBeginPlay
  ;[1 1 1] setting the coordinates of the zone center(var1)
  (Variables|Default|SetCurrentObjectLocation (Transformation|GetWorldLocation (Variables|Default|GetCube)))
  (CallFunction|MovetoTarget))

(fn ConstructionScript)

(fn IsActorinBoundires2D
  (params (MIN_X :type Float%20%28double-precision%29) (MAX_X :type Float%20%28double-precision%29) (MIN_Y :type Float%20%28double-precision%29) (MAX_Y :type Float%20%28double-precision%29))
  (bind _returnvalue (Transformation|GetActorLocation))
  (bind _currentobjectlocation (Variables|Default|GetCurrentObjectLocation))
  ;[1 1 1] Settings coordinats zone
  (return (and (Math|Float|InRange(Float) (.x _returnvalue) (+ MIN_X (.x _currentobjectlocation)) (+ MAX_X (.x _currentobjectlocation))) (Math|Float|InRange(Float) (.y _returnvalue) (+ MIN_Y (.y _currentobjectlocation)) (+ MAX_Y (.y _currentobjectlocation))))))